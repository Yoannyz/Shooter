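; GM_Game is the game mode that runs enemy spawning and player respawning.
; On BeginPlay it finds the first BP_EnemySpawner and starts a looping timer that calls its SpawnEnemy function by name.
; RespawnPlayer destroys every BP_Enemy, spawns a new BP_Player at a stored transform and has the first player controller possess it.
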(event Custom|RespawnPlayer
  (bind _outactors (Actor|GetAllActorsOfClass "/Game/Blueprints/BP_Enemy.BP_Enemy_C"))
  (for _array_element _outactors
    (Actor|DestroyActor _array_element))
  (bind _returnvalue (Game|SpawnActorfromClass "/Game/Blueprints/BP_Player.BP_Player_C" (Variables|Default|GetSpawnTransform) "AdjustIfPossibleButAlwaysSpawn" 0 0))
  (Pawn|Possess (Game|GetPlayerController 0) _returnvalue))

(event EventBeginPlay
  (bind _outactors (Actor|GetAllActorsOfClass "/Game/Blueprints/BP_EnemySpawner.BP_EnemySpawner_C"))
  (bind _output_get (Variables|Default|SetEnemySpawner (Utilities|Array|Get(acopy) _outactors)))
  (Utilities|Time|SetTimerbyFunctionName _output_get "SpawnEnemy" 2.0 true))

(fn ConstructionScript)