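; Player pawn for a twin-stick style shooter, with world-axis movement and look input that both aims and fires.
; Both look axes share one branch: past a dead zone it sets control rotation and pulls the weapon trigger, otherwise it releases it.
; BeginPlay records the spawn transform in GM_Game and attaches a spawned BP_Gun to the mesh's GunSocket.
; Lethal damage destroys pawn and gun after a delay, then requests a respawn from GM_Game.
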(event EventBeginPlay
  (bind _mesh (Variables|Character|GetMesh))
  (Utilities|FlowControl|Sequence
    (:then_0
      (bind _asgm_game (Utilities|Casting|CastToGM_Game (Game|GetGameMode)))
      (bind _output_get (Variables|Default|SetGameMode _asgm_game))
      (Variables|/Game/Blueprints/GM_Game.GM_Game_C|SetSpawnTransform _output_get (Transformation|GetActorTransform)))
    (:then_1
      (bind _returnvalue (Game|SpawnActorfromClass "/Game/Blueprints/BP_Gun.BP_Gun_C" (Transformation|GetSocketTransform _mesh "GunSocket" "RTS_World") "Undefined" 0 0))
      (bind _output_get_2 (Variables|Default|SetWeapon _returnvalue))
      (Transformation|AttachComponentToComponent _output_get_2 _mesh "GunSocket" "SnapToTarget" "KeepRelative" "KeepWorld" true))))

(event EventApplyDamage
  (params (Damage :type Float%20%28single-precision%29))
  (bind _output_get (Variables|Default|SetHealth (- (Variables|Default|GetHealth) Damage)))
  (Development|PrintString (Utilities|String|ToString(Float) _output_get))
  (bind _output_get_2 (Variables|Default|SetIsDead (<= _output_get 0.0)))
  (if _output_get_2
    (Utilities|FlowControl|Delay 2.0)
    (Actor|DestroyActor self)
    (Default|RespawnPlayer (Variables|Default|GetGameMode))))

(event Input|AxisEvents|InputAxisMoveForward
  (params (AxisValue :type Float%20%28single-precision%29))
  (Pawn|Input|AddMovementInput "1.000000, 0, 0" AxisValue false))

(event Input|AxisEvents|InputAxisMoveRight
  (params (AxisValue :type Float%20%28single-precision%29))
  (Pawn|Input|AddMovementInput "0.000000,1.000000, 0" AxisValue false))

(event Input|AxisEvents|InputAxisLookForward
  (params (AxisValue :type Float%20%28single-precision%29))
  (bind _weapon (Variables|Default|GetWeapon))
  (if (>= (Math|Vector|VectorLength (Math|Vector|MakeVector AxisValue (stale Input|AxisEvents|InputAxisLookRightAxis AxisValue) 0.0)) 0.2)
    (Pawn|SetControlRotation (Pawn|GetController) (Math|Rotator|MakeRotfromX (Math|Vector|MakeVector AxisValue (stale Input|AxisEvents|InputAxisLookRightAxis AxisValue) 0.0)))
    (Default|PullTrigger _weapon)
    (else
      (Default|ReleaseTrigger _weapon))))

(event Input|AxisEvents|InputAxisLookRightAxis
  (params (AxisValue :type Float%20%28single-precision%29))
  (bind _weapon (Variables|Default|GetWeapon))
  (if (>= (Math|Vector|VectorLength (Math|Vector|MakeVector (stale Input|AxisEvents|InputAxisLookForward AxisValue) AxisValue 0.0)) 0.2)
    (Pawn|SetControlRotation (Pawn|GetController) (Math|Rotator|MakeRotfromX (Math|Vector|MakeVector (stale Input|AxisEvents|InputAxisLookForward AxisValue) AxisValue 0.0)))
    (Default|PullTrigger _weapon)
    (else
      (Default|ReleaseTrigger _weapon))))

(fn ConstructionScript)