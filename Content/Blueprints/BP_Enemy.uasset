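; BP_Enemy is an enemy that deals repeated damage to an overlapping BP_Player and can itself be killed.
; Overlap starts a looping timer that calls ApplyDamage on the player, and end overlap clears it by function name.
; Its own ApplyDamage lowers Health, sets IsDead at zero or below, detaches the controller and destroys the actor after a delay.
; The construction script tints the mesh with BodyColor through a dynamic material instance.
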(event Custom|DamagePlayer
  (Default|ApplyDamage (Variables|Default|GetPlayer) (Variables|Default|GetDamage)))

(event EventApplyDamage
  (params (Damage :type Float%20%28single-precision%29))
  (bind _output_get (Variables|Default|SetHealth (- (Variables|Default|GetHealth) Damage)))
  (bind _output_get_2 (Variables|Default|SetIsDead (<= _output_get 0.0)))
  (if _output_get_2
    (Class|Pawn|DetachfromControllerPendingDestroy)
    (Utilities|FlowControl|Delay 2.0)
    (Actor|DestroyActor)))

(event Collision|EventActorBeginOverlap
  (params (OtherActor :type Actor%20Object%20Reference))
  (bind _asbp_player (Utilities|Casting|CastToBP_Player OtherActor))
  (Variables|Default|SetPlayer _asbp_player)
  (Utilities|Time|SetTimerbyEvent (delegate Custom|DamagePlayer) 0.5 true))

(event Collision|EventActorEndOverlap
  (params (OtherActor :type Actor%20Object%20Reference))
  (if (== OtherActor (Variables|Default|GetPlayer))
    (Utilities|Time|ClearTimerbyFunctionName 0 "DamagePlayer")))

(fn ConstructionScript
  (bind _returnvalue (Rendering|Material|CreateDynamicMaterialInstance (Variables|Character|GetMesh) 0 0 "None" :!class /Script/Engine.PrimitiveComponent))
  (Rendering|Material|SetVectorParameterValue _returnvalue "BodyColor" (Variables|Default|GetBodyColor) :!class /Script/Engine.MaterialInstanceDynamic))